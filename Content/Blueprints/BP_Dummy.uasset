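; BP_Dummy is a stealth takedown victim that shows a prompt widget while BP_ThirdPersonCharacter overlaps its TakeDownRadius.
; The widget turns each Tick to face the player camera.
; StealthBackAssasin plays the victim's paired knife montage, hides the prompt, and returns the AssasinRef location and dummy rotation.
; It also triggers RagDoll, which uses fixed delays to play a death sound and then enable mesh physics simulation.
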(event OnComponentBeginOverlap(TakeDownRadius)
  (params (OverlappedComponent :type Primitive%20Component%20Object%20Reference) (OtherActor :type Actor%20Object%20Reference) (OtherComp :type Primitive%20Component%20Object%20Reference) (OtherBodyIndex :type Integer) (bFromSweep :type Boolean) (SweepResult :type Hit%20Result%20Structure%20%28by%20ref%29))
  (Utilities|Casting|CastToBP_ThirdPersonCharacter OtherActor)
  (Rendering|SetVisibility (Variables|Default|GetTakeDown%20Widget) true false))

(event OnComponentEndOverlap(TakeDownRadius)
  (params (OverlappedComponent :type Primitive%20Component%20Object%20Reference) (OtherActor :type Actor%20Object%20Reference) (OtherComp :type Primitive%20Component%20Object%20Reference) (OtherBodyIndex :type Integer))
  (Utilities|Casting|CastToBP_ThirdPersonCharacter OtherActor)
  (Rendering|SetVisibility (Variables|Default|GetTakeDown%20Widget) false false))

(event Custom|RagDoll
  ;[1 1 1] RagDoll
  (Utilities|FlowControl|Sequence
    (:then_0
      (Utilities|FlowControl|Delay 2.5)
      (Physics|SetSimulatePhysics (Variables|Character|GetMesh) true))
    (:then_1
      (Utilities|FlowControl|Delay 1.8)
      (Audio|PlaySoundatLocation "/Game/Audio/Grunts_and_Hits/SC_Death_SFX.SC_Death_SFX" (Transformation|GetActorLocation) "0, 0, 0" 1.0 1.0 0.0 "/Game/Audio/SA_Character.SA_Character" 0 0 0))))

(event EventBeginPlay)

(event Collision|EventActorBeginOverlap
  (params (OtherActor :type Actor%20Object%20Reference)))

(event EventTick
  (params (DeltaSeconds :type Float%20%28single-precision%29))
  (Transformation|SetWorldRotation (Variables|Default|GetTakeDown%20Widget) (Math|Rotator|FindLookatRotation (Transformation|GetWorldLocation (Variables|Default|GetTakeDown%20Widget)) (Transformation|GetWorldLocation (Variables|/Script/Engine.PlayerCameraManager|GetTransformComponent (Game|GetPlayerCameraManager 0)))) false false))

(fn ConstructionScript)

(fn StealthBackAssasin
  (Animation|PlayAnimMontage "/Game/Characters/MC_Character/Animations/Assasination/Paired_Knife_Stealth_KidneyAndNeck_Vic_Montage.Paired_Knife_Stealth_KidneyAndNeck_Vic_Montage" 1.0 "None")
  (CallFunction|RagDoll)
  (Rendering|SetVisibility (Variables|Default|GetTakeDown%20Widget) false false)
  (return (Transformation|GetWorldLocation (Variables|Default|GetAssasinRef)) (Transformation|GetActorRotation)))