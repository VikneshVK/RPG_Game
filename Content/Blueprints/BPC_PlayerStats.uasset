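; Player stats component for BP_ThirdPersonCharacter that tracks health, stamina, EXP and level.
; Each change function updates the value and writes it straight to the character's HUD widget, which is first filled one tick after BeginPlay.
; Decrease functions return true on depletion, and health and stamina gains clamp to their maximums.
; Reaching max EXP triggers a level-up that raises the EXP cap, resets EXP without carrying overflow and plays sounds.
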(event EventBeginPlay
  (Utilities|FlowControl|DelayUntilNextTick)
  (bind _asbp_third_person_character (Utilities|Casting|CastToBP_ThirdPersonCharacter (Components|GetOwner)))
  (Variables|Default|SetPlayer%20Character%20BP _asbp_third_person_character)
  (Progress|SetPercent (Variables|/Game/UI/WBP_HUD.WBP_HUD_C|GetStaminabar (Variables|/Game/ThirdPerson/Blueprints/BP_ThirdPersonCharacter.BP_ThirdPersonCharacter_C|GetHUD%20%20Widget (Variables|Default|GetPlayer%20Character%20BP))) (/ (Variables|Energy|GetCurrent%20Stamina) (Variables|Energy|GetMax%20Stamina)))
  (Progress|SetPercent (Variables|/Game/UI/WBP_HUD.WBP_HUD_C|GetHealthBar (Variables|/Game/ThirdPerson/Blueprints/BP_ThirdPersonCharacter.BP_ThirdPersonCharacter_C|GetHUD%20%20Widget (Variables|Default|GetPlayer%20Character%20BP))) (/ (Variables|Health|GetCurrent%20Health) (Variables|Health|GetMax%20Health)))
  (Rendering|Components|TextRender|SetText (Variables|/Game/UI/WBP_HUD.WBP_HUD_C|GetHealth_Text (Variables|/Game/ThirdPerson/Blueprints/BP_ThirdPersonCharacter.BP_ThirdPersonCharacter_C|GetHUD%20%20Widget (Variables|Default|GetPlayer%20Character%20BP))) (Utilities|Text|ToText(Float) (Variables|Health|GetCurrent%20Health) "HalfToEven"))
  (Progress|SetPercent (Variables|/Game/UI/WBP_HUD.WBP_HUD_C|GetEXPBar (Variables|/Game/ThirdPerson/Blueprints/BP_ThirdPersonCharacter.BP_ThirdPersonCharacter_C|GetHUD%20%20Widget (Variables|Default|GetPlayer%20Character%20BP))) (/ (Variables|EXPandLevel|GetEXP) (Variables|EXPandLevel|GetMax%20EXP)))
  (Rendering|Components|TextRender|SetText (Variables|/Game/UI/WBP_HUD.WBP_HUD_C|GetEXPText (Variables|/Game/ThirdPerson/Blueprints/BP_ThirdPersonCharacter.BP_ThirdPersonCharacter_C|GetHUD%20%20Widget (Variables|Default|GetPlayer%20Character%20BP))) (Utilities|Text|FormatText "{Current EXP}/ {Max EXP} " (Variables|EXPandLevel|GetEXP) (Variables|EXPandLevel|GetMax%20EXP)))
  (Rendering|Components|TextRender|SetText (Variables|/Game/UI/WBP_HUD.WBP_HUD_C|GetLevelText (Variables|/Game/ThirdPerson/Blueprints/BP_ThirdPersonCharacter.BP_ThirdPersonCharacter_C|GetHUD%20%20Widget (Variables|Default|GetPlayer%20Character%20BP))) (Utilities|Text|ToText(Integer) (Variables|EXPandLevel|GetLevel))))

(fn DecreaseHealth
  (params (Damage :type Float%20%28double-precision%29))
  (bind _player_character_bp (Variables|Default|GetPlayer%20Character%20BP))
  (bind _hud__widget (Variables|/Game/ThirdPerson/Blueprints/BP_ThirdPersonCharacter.BP_ThirdPersonCharacter_C|GetHUD%20%20Widget _player_character_bp))
  (if (not (<= (Variables|Health|GetCurrent%20Health) 0.0))
    (bind _output_get (Variables|Health|SetCurrent%20Health (- (Variables|Health|GetCurrent%20Health) Damage)))
    (Progress|SetPercent (Variables|/Game/UI/WBP_HUD.WBP_HUD_C|GetHealthBar _hud__widget) (/ _output_get (Variables|Health|GetMax%20Health)))
    (Rendering|Components|TextRender|SetText (Variables|/Game/UI/WBP_HUD.WBP_HUD_C|GetHealth_Text _hud__widget) (Utilities|Text|ToText(Float) (Variables|Health|GetCurrent%20Health) "HalfToEven"))
    (if (<= (Variables|Health|GetCurrent%20Health) 0.0)
      _
      (else
        (return false))))
  (return true))

(fn IncreaseMaxHealth
  (params (Increased_value :type Float%20%28double-precision%29))
  (bind _player_character_bp (Variables|Default|GetPlayer%20Character%20BP))
  (bind _hud__widget (Variables|/Game/ThirdPerson/Blueprints/BP_ThirdPersonCharacter.BP_ThirdPersonCharacter_C|GetHUD%20%20Widget _player_character_bp))
  (Variables|Health|SetMax%20Health (+ (Variables|Health|GetMax%20Health) Increased_value))
  (Progress|SetPercent (Variables|/Game/UI/WBP_HUD.WBP_HUD_C|GetHealthBar _hud__widget) (/ (Variables|Health|GetCurrent%20Health) (Variables|Health|GetMax%20Health)))
  (Rendering|Components|TextRender|SetText (Variables|/Game/UI/WBP_HUD.WBP_HUD_C|GetHealth_Text _hud__widget) (Utilities|Text|ToText(Float) (Variables|Health|GetCurrent%20Health) "HalfToEven")))

(fn DecreaseStamina
  (params (Stamina%20needed :type Float%20%28double-precision%29))
  (if (not (<= (Variables|Energy|GetCurrent%20Stamina) 0.0))
    (Variables|Energy|SetCurrent%20Stamina (- (Variables|Energy|GetCurrent%20Stamina) Stamina%20needed))
    (Progress|SetPercent (Variables|/Game/UI/WBP_HUD.WBP_HUD_C|GetStaminabar (Variables|/Game/ThirdPerson/Blueprints/BP_ThirdPersonCharacter.BP_ThirdPersonCharacter_C|GetHUD%20%20Widget (Variables|Default|GetPlayer%20Character%20BP))) (/ (Variables|Energy|GetCurrent%20Stamina) (Variables|Energy|GetMax%20Stamina)))
    (if (<= (Variables|Energy|GetCurrent%20Stamina) 0.0)
      _
      (else
        (return false))))
  (return true))

(fn IncreaseMaxStamina
  (params (increased_value :type Float%20%28double-precision%29))
  (Variables|Energy|SetMax%20Stamina (+ (Variables|Energy|GetMax%20Stamina) increased_value))
  (Progress|SetPercent (Variables|/Game/UI/WBP_HUD.WBP_HUD_C|GetStaminabar (Variables|/Game/ThirdPerson/Blueprints/BP_ThirdPersonCharacter.BP_ThirdPersonCharacter_C|GetHUD%20%20Widget (Variables|Default|GetPlayer%20Character%20BP))) (/ (Variables|Energy|GetCurrent%20Stamina) (Variables|Energy|GetMax%20Stamina))))

(fn IncreaseHealth
  (params (Increased%20value :type Float%20%28double-precision%29))
  (bind _player_character_bp (Variables|Default|GetPlayer%20Character%20BP))
  (bind _hud__widget (Variables|/Game/ThirdPerson/Blueprints/BP_ThirdPersonCharacter.BP_ThirdPersonCharacter_C|GetHUD%20%20Widget _player_character_bp))
  (Variables|Health|SetCurrent%20Health (+ (Variables|Health|GetCurrent%20Health) Increased%20value))
  (if (>= (Variables|Health|GetCurrent%20Health) (Variables|Health|GetMax%20Health))
    (Variables|Health|SetCurrent%20Health (Variables|Health|GetMax%20Health)))
  (Progress|SetPercent (Variables|/Game/UI/WBP_HUD.WBP_HUD_C|GetHealthBar _hud__widget) (/ (Variables|Health|GetCurrent%20Health) (Variables|Health|GetMax%20Health)))
  (Rendering|Components|TextRender|SetText (Variables|/Game/UI/WBP_HUD.WBP_HUD_C|GetHealth_Text _hud__widget) (Utilities|Text|ToText(Float) (Variables|Health|GetCurrent%20Health) "HalfToEven")))

(fn IncreaseStamina
  (params (Increased%20Value :type Float%20%28double-precision%29))
  (Variables|Energy|SetCurrent%20Stamina (+ (Variables|Energy|GetCurrent%20Stamina) Increased%20Value))
  (if (>= (Variables|Energy|GetCurrent%20Stamina) (Variables|Energy|GetMax%20Stamina))
    (Variables|Energy|SetCurrent%20Stamina (Variables|Energy|GetMax%20Stamina)))
  (Progress|SetPercent (Variables|/Game/UI/WBP_HUD.WBP_HUD_C|GetStaminabar (Variables|/Game/ThirdPerson/Blueprints/BP_ThirdPersonCharacter.BP_ThirdPersonCharacter_C|GetHUD%20%20Widget (Variables|Default|GetPlayer%20Character%20BP))) (/ (Variables|Energy|GetCurrent%20Stamina) (Variables|Energy|GetMax%20Stamina))))

(fn IncreaseEXP
  (params (Added%20EXP :type Float%20%28double-precision%29))
  (Variables|EXPandLevel|SetEXP (+ (Variables|EXPandLevel|GetEXP) Added%20EXP))
  (if (>= (Variables|EXPandLevel|GetEXP) (Variables|EXPandLevel|GetMax%20EXP))
    (EXPandLevel|IncreaseLevel 1))
  (Progress|SetPercent (Variables|/Game/UI/WBP_HUD.WBP_HUD_C|GetEXPBar (Variables|/Game/ThirdPerson/Blueprints/BP_ThirdPersonCharacter.BP_ThirdPersonCharacter_C|GetHUD%20%20Widget (Variables|Default|GetPlayer%20Character%20BP))) (/ (Variables|EXPandLevel|GetEXP) (Variables|EXPandLevel|GetMax%20EXP)))
  (Rendering|Components|TextRender|SetText (Variables|/Game/UI/WBP_HUD.WBP_HUD_C|GetEXPText (Variables|/Game/ThirdPerson/Blueprints/BP_ThirdPersonCharacter.BP_ThirdPersonCharacter_C|GetHUD%20%20Widget (Variables|Default|GetPlayer%20Character%20BP))) (Utilities|Text|FormatText "{Current EXP}/ {Max EXP} " (Variables|EXPandLevel|GetEXP) (Variables|EXPandLevel|GetMax%20EXP))))

(fn IncreaseLevel
  (params (Added%20Level :type Integer))
  (Variables|EXPandLevel|SetLevel (+ (Variables|EXPandLevel|GetLevel) Added%20Level))
  (Variables|EXPandLevel|SetMax%20EXP (+ (Variables|EXPandLevel|GetMax%20EXP) 1.5e+02))
  (Variables|EXPandLevel|SetEXP 0.0)
  (Rendering|Components|TextRender|SetText (Variables|/Game/UI/WBP_HUD.WBP_HUD_C|GetLevelText (Variables|/Game/ThirdPerson/Blueprints/BP_ThirdPersonCharacter.BP_ThirdPersonCharacter_C|GetHUD%20%20Widget (Variables|Default|GetPlayer%20Character%20BP))) (Utilities|Text|ToText(Integer) (Variables|EXPandLevel|GetLevel)))
  (Audio|PlaySound2D "/Game/Audio/UI/epic-level-up.epic-level-up" 1.0 1.0 0.0 0 0)
  (Audio|PlaySound2D "/Game/Audio/UI/542825__kostas17__magic-spell.542825__kostas17__magic-spell" 1.0 1.0 0.0 0 0))